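; Enemy spawner actor that spawns a group of enemies when the first player pawn enters its Trigger volume.
; On overlap, it spawns AmountToSpawn Bp_enemey actors at random XY points within the Location box extent, at that component's world Z.
; Spawning requires SpawnedActors to be empty, but this graph never adds the spawned enemies to it, so re-entering the trigger can spawn again.
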(event OnComponentBeginOverlap(Trigger)
  (params (OverlappedComponent :type Primitive%20Component%20Object%20Reference) (OtherActor :type Actor%20Object%20Reference) (OtherComp :type Primitive%20Component%20Object%20Reference) (OtherBodyIndex :type Integer) (bFromSweep :type Boolean) (SweepResult :type Hit%20Result%20Structure%20%28by%20ref%29))
  (bind _location (Variables|Default|GetLocation))
  (bind _returnvalue (Transformation|GetWorldLocation _location))
  (bind _boxextent (Variables|/Script/Engine.BoxComponent|GetBoxExtent _location))
  (if (and (== OtherActor (Game|Player|GetPlayerPawn 0)) (Utilities|Array|IsEmpty (Variables|Default|GetspawnedActors)))
    (for _index (range 1 (Variables|Default|GetamountToSpawn))
      (Game|SpawnActorfromClass "/Game/enemey/bp_enemey.bp_enemey_C" (Math|Transform|MakeTransform (Math|Vector|MakeVector (Math|Random|RandomFloatinRange (- (.x _returnvalue) (.x _boxextent)) (+ (.x _returnvalue) (.x _boxextent))) (Math|Random|RandomFloatinRange (- (.y _returnvalue) (.y _boxextent)) (+ (.y _returnvalue) (.y _boxextent))) (.z _returnvalue)) "0, 0, 0" "1.000000,1.000000,1.000000") "Undefined" "MultiplyWithRoot" 0 0))))

(fn ConstructionScript)