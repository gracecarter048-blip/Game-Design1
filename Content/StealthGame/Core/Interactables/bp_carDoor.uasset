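; Car door interactable that acts as the level's win point, checking the overlapping player character's key count.
; With more than one key, it subtracts three, plays an engine sound, destroys the door, calls the character's YouwinCheckpoint and immediately quits the game.
; Otherwise it prints a locked-door message.
; Box collision events enable input, though end-overlap casts the other actor to the game mode instead of the character.
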(event OnComponentBeginOverlap(Boxcollision)
  (params (OverlappedComponent :type Primitive%20Component%20Object%20Reference) (OtherActor :type Actor%20Object%20Reference) (OtherComp :type Primitive%20Component%20Object%20Reference) (OtherBodyIndex :type Integer) (bFromSweep :type Boolean) (SweepResult :type Hit%20Result%20Structure%20%28by%20ref%29))
  (Utilities|Casting|CastToBP_ThirdPersonCharacterCustom OtherActor)
  (Input|EnableInput (Game|GetPlayerController 0)))

(event OnComponentEndOverlap(Boxcollision)
  (params (OverlappedComponent :type Primitive%20Component%20Object%20Reference) (OtherActor :type Actor%20Object%20Reference) (OtherComp :type Primitive%20Component%20Object%20Reference) (OtherBodyIndex :type Integer))
  (Utilities|Casting|CastToBP_ThirdPersonGameModeCustom OtherActor)
  (Input|EnableInput (Game|GetPlayerController 0)))

(event Collision|EventActorBeginOverlap
  (params (OtherActor :type Actor%20Object%20Reference))
  (bind _asbp_third_person_character_custom (Utilities|Casting|CastToBP_ThirdPersonCharacterCustom OtherActor))
  (Variables|Default|SetCharacter%20Ref _asbp_third_person_character_custom)
  (if (> (Variables|/Game/StealthGame/Core/Characters/PlayerCharacter/BP_ThirdPersonCharacterCustom.BP_ThirdPersonCharacterCustom_C|GetKey%20Count _asbp_third_person_character_custom) 1) ; Like an If Statement
    (Variables|/Game/StealthGame/Core/Characters/PlayerCharacter/BP_ThirdPersonCharacterCustom.BP_ThirdPersonCharacterCustom_C|SetKey%20Count _asbp_third_person_character_custom (- (Variables|/Game/StealthGame/Core/Characters/PlayerCharacter/BP_ThirdPersonCharacterCustom.BP_ThirdPersonCharacterCustom_C|GetKey%20Count _asbp_third_person_character_custom) 3)) ; Remove a Key, then open door.
    (Audio|PlaySound2D "/Game/developer/audio/car/carEngine.carEngine" 1.0 1.0 0.0 0 0)
    (Components|DestroyComponent (Variables|Default|GetDoor))
    (Default|YouwinCheckpoint (Variables|Default|GetCharacter%20Ref))
    (Game|QuitGame 0 "Quit" false)
    (else
      (Development|PrintString "Get More Keys! Door is locked" true true "(R=0.479167,G=0.051103,B=0.000000,A=1.000000)" 5.0))))

(fn ConstructionScript)