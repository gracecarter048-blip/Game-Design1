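; Enemy AI character that patrols target points or wanders randomly, then chases and punches the player on sight.
; Tick picks AIMoveTo behaviours, gated by CanMove and PlayerVisable; PawnSensing handles sight, turning it red and larger, and investigates noises.
; The montage notify sphere-traces from the right hand, sending a hit player to their checkpoint, while misses re-arm the attack.
; EnableRagdoll destroys it after a delay.
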(event OnSeePawn(PawnSensing)
  (params (Pawn :type Pawn%20Object%20Reference))
  (if true
    (Utilities|Casting|CastToBP_ThirdPersonCharacterCustom Pawn
      (:then
        (Transformation|SetActorScale3D "1.250000,1.250000,1.250000")
        (Rendering|Material|SetMaterial (Variables|Character|GetMesh) 0 "/AnimationSharing/AnimSharingRed.AnimSharingRed")
        (Variables|Default|SetbPlayerVisable true))
      (:CastFailed
        (Variables|Default|SetbPlayerVisable false)))
    (else
      (Utilities|FlowControl|RetriggerableDelay 2.0)
      (Variables|Default|SetbPlayerVisable false)
      (Rendering|Material|SetMaterial (Variables|Character|GetMesh) 0 0)
      (Transformation|SetActorScale3D "1.000000,1.000000,1.000000")
      (CallFunction|MovetoNextPatrolPoint))))

(event OnHearNoise(PawnSensing)
  (params (Instigator :type Pawn%20Object%20Reference) (Location :type Vector%20%28by%20ref%29 :default "0, 0, 0") (Volume :type Float%20%28single-precision%29))
  (CallFunction|UpdateWalkSpeed 3e+02)
  (Variables|Default|SetbCanMove true)
  (AI|AIMoveTo self Location Instigator 5.0 false
    (:OnSuccess
      _)
    (:OnFail
      _))
  (Utilities|FlowControl|Delay 12.0)
  (Rendering|Material|SetMaterial (Variables|Character|GetMesh) 0 "/Game/StealthGame/Core/Characters/PlayerCharacter/Mannequins/Materials/Instances/Quinn/MI_Quinn_02.MI_Quinn_02")
  (Transformation|SetActorScale3D "1.000000,1.000000,1.000000")
  (Variables|Default|SetbCanMove true)
  (CallFunction|ControlRandom))

(event Custom|ChasePlayer
  (CallFunction|UpdateWalkSpeed 6e+02)
  (Variables|Default|SetbCanMove false)
  (AI|AIMoveTo self "0, 0, 0" (Game|GetPlayerCharacter 0) 75.0 false
    (:OnSuccess
      (CallFunction|Attack)
      (Rendering|Material|SetMaterial (Variables|Character|GetMesh) 0 0)
      (Transformation|SetActorScale3D "1.000000,1.000000,1.000000")
      (Variables|Default|SetbCanMove true)
      (CallFunction|ControlRandom))))

(event Custom|Attack
  (bind _mesh (Variables|Character|GetMesh))
  (bind _returnvalue (Transformation|GetSocketLocation _mesh "hand_r"))
  ;[0.15 0.1407 0.04319 0.5] Bonk
  (Utilities|FlowControl|DoOnce false ; Only Reset Attack on miss.
    (:Completed
      (bind _notifyname (Animation|Montage|PlayMontage (Variables|Character|GetMesh) "/Game/StealthGame/Characters/Enemies/AM_Attack_01.AM_Attack_01") ; Play the AM_Attack_01
        (:OnCompleted
          (if (Variables|Default|GetbHostile) ; Keep attacking if you haven't landed the hit.
            (CallFunction|ResetAttack)))
        (:OnNotifyBegin
          (Audio|PlaySound2D "/Game/developer/audio/punch/punch2.punch2" 1.0 1.0 0.0 0 0)
          (switch name _notifyname ; Pick the proper attack type(standard when there is more than one type of attack)
            (:AttackDamage
              (bind (_outhits _returnvalue_2) (Collision|MultiSphereTraceForObjects _returnvalue (+ _returnvalue (* (Transformation|GetActorForwardVector) (Variables|Default|GetMeleeTraceDistance))) (Variables|Default|GetMeleeTraceRadius) (Utilities|Array|MakeArray "ObjectTypeQuery3") false 0 "None")) ; Trace forward from hand socket.
              (if _returnvalue_2 ; If a pawn is hit in that trace...
                (for _array_element _outhits ; ...loop through the results....
                  (bind _asbp_third_person_character_custom (Utilities|Casting|CastToBP_ThirdPersonCharacterCustom (.HitActor (Collision|BreakHitResult _array_element))))
                  (Default|LoadCheckpoint _asbp_third_person_character_custom)
                  (Variables|Default|SetbHostile false) ; ...and stop attacking...
                )))))))))

(event Custom|MoveToNextPatrolPoint
  (CallFunction|UpdateWalkSpeed 2e+02)
  (Variables|Default|SetbCanMove false)
  (AI|AIMoveTo self "0, 0, 0" (Utilities|Array|Get(acopy) (Variables|Default|GetTargetPoints) (Variables|Default|GetpatrolTargetPointIndex)) 5.0 false
    (:OnSuccess
      (CallFunction|SetNextPatrolPointIndex)
      (Utilities|FlowControl|Delay 3.0)
      (Variables|Default|SetbCanMove true))))

(event Custom|ResetAttack
  (bind _mesh (Variables|Character|GetMesh))
  (bind _returnvalue (Transformation|GetSocketLocation _mesh "hand_r"))
  ;[0.15 0.1407 0.04319 0.5] Bonk
  (Utilities|FlowControl|DoOnce false) ; enters at Reset
)

(event Custom|EnableRagdoll
  (bind _mesh (Variables|Character|GetMesh))
  (if true
    (Physics|SetSimulatePhysics _mesh true)
    (Collision|SetCollisionProfileName _mesh "ragdoll" true :!class /Script/Engine.PrimitiveComponent)
    (Animation|StopAnimMontage 0)
    (Variables|Default|SetbCanMove false)
    (Utilities|FlowControl|Delay 3.0)
    (Actor|DestroyActor)))

(event Custom|control%20random
  (CallFunction|UpdateWalkSpeed 2e+02)
  (Variables|Default|SetbCanMove false)
  (AI|AIMoveTo self (.RandomLocation (AI|Navigation|GetRandomReachablePointinRadius (Transformation|GetActorLocation) 2e+03 0 0)) 0 5e+01 false
    (:OnSuccess
      (Utilities|FlowControl|Delay 1.5)
      (Variables|Default|SetbCanMove true))))

(event Custom|SetNextPatrolPointIndex
  (Variables|Default|SetpatrolTargetPointIndex (Math|Integer|%(Integer) (+ (Variables|Default|GetpatrolTargetPointIndex) (Utilities|Array|Length (Variables|Default|GetTargetPoints))) 1)))

(event EventBeginPlay)

(event EventTick
  (params (DeltaSeconds :type Float%20%28single-precision%29))
  (bind _bplayervisable (Variables|Default|GetbPlayerVisable))
  (if (Variables|Default|GetbCanMove)
    (if _bplayervisable
      (CallFunction|ChasePlayer)
      (elif (Variables|Default|GetTargetPointMovement)
        (CallFunction|MovetoNextPatrolPoint)
        (else
          (CallFunction|ControlRandom))))
    (elif _bplayervisable
      (CallFunction|ChasePlayer))))

(fn ConstructionScript)

(fn UpdateWalkSpeed
  (params (NewWalkSpeed :type Float%20%28double-precision%29))
  (Variables|/Script/Engine.CharacterMovementComponent|SetMaxWalkSpeed (Variables|Character|GetCharacterMovement) NewWalkSpeed))