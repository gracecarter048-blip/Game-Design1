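; Alien spawner trigger actor that spawns a single enemy when the player walks into it.
; BeginPlay caches the player as BP_ThirdPersonCharacterCustom, and the Capsule's begin overlap checks against that reference.
; A DoOnce gate limits the trigger to one call of alienSpwaner, which spawns Bp_enemey1 at the Billboard's transform, adjusting for collisions, with the player set as Instigator.
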(event OnComponentBeginOverlap(Capsule)
  (params (OverlappedComponent :type Primitive%20Component%20Object%20Reference) (OtherActor :type Actor%20Object%20Reference) (OtherComp :type Primitive%20Component%20Object%20Reference) (OtherBodyIndex :type Integer) (bFromSweep :type Boolean) (SweepResult :type Hit%20Result%20Structure%20%28by%20ref%29))
  (if (== OtherActor (Variables|Default|GetAs%20BP%20Third%20Person%20Character%20Custom))
    (Utilities|FlowControl|DoOnce false
      (:Completed
        (CallFunction|AlienSpwaner)))))

(event Custom|alienSpwaner
  (Game|SpawnActorfromClass "/Game/enemey/bp_enemey1.bp_enemey1_C" (Transformation|GetWorldTransform (Variables|Default|GetBillboard)) "AdjustIfPossibleButAlwaysSpawn" "MultiplyWithRoot" 0 (Game|GetPlayerCharacter 0)))

(event EventBeginPlay
  (bind _asbp_third_person_character_custom (Utilities|Casting|CastToBP_ThirdPersonCharacterCustom (Game|GetPlayerCharacter 0)))
  (Variables|Default|SetAs%20BP%20Third%20Person%20Character%20Custom _asbp_third_person_character_custom))

(fn ConstructionScript)