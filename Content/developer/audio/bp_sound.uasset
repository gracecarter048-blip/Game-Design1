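; A placeable sound trigger that plays a sound when the custom third-person character enters its sphere.
; The construction script applies the exposed sound, attenuation settings and sphere radius to the Audio and Sphere components.
; On overlap, playback starts at a random offset within the sound's duration, and nothing in the graph stops it on exit.
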(event OnComponentBeginOverlap(Sphere)
  (params (OverlappedComponent :type Primitive%20Component%20Object%20Reference) (OtherActor :type Actor%20Object%20Reference) (OtherComp :type Primitive%20Component%20Object%20Reference) (OtherBodyIndex :type Integer) (bFromSweep :type Boolean) (SweepResult :type Hit%20Result%20Structure%20%28by%20ref%29))
  (Utilities|Casting|CastToBP_ThirdPersonCharacterCustom OtherActor)
  (Audio|Components|Audio|Play (Variables|Default|GetAudio) (Math|Random|RandomFloatinRange 0.0 (Variables|/Script/Engine.SoundBase|GetDuration (Variables|Default|GetsoundQue)))))

(fn ConstructionScript
  (Audio|Components|Audio|SetSound (Variables|Default|GetAudio) (Variables|Default|GetsoundQue))
  (Variables|/Script/Engine.AudioComponent|SetAttenuationSettings (Variables|Default|GetAudio) (Variables|Default|GetsoundAlteration))
  (Components|Sphere|SetSphereRadius (Variables|Default|GetSphere) (Variables|Default|GetsphereRadius) true))