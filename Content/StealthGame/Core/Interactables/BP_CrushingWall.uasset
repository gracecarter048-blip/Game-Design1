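; BP_CrushingWall is a moving wall hazard that loads the game state when the custom third-person character touches it.
; From BeginPlay, a Timeline lerps the Wall between the relative locations of the Begin and End components, without sweep.
; On each finish, a short delay and FlipFlop alternate reversing and replaying the Timeline, so the wall oscillates continuously.
; Overlap with the Wall casts the other actor to BP_ThirdPersonCharacterCustom and calls its LoadGameState.
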(event OnComponentBeginOverlap(wall)
  (params (OverlappedComponent :type Primitive%20Component%20Object%20Reference) (OtherActor :type Actor%20Object%20Reference) (OtherComp :type Primitive%20Component%20Object%20Reference) (OtherBodyIndex :type Integer) (bFromSweep :type Boolean) (SweepResult :type Hit%20Result%20Structure%20%28by%20ref%29))
  (bind _asbp_third_person_character_custom (Utilities|Casting|CastToBP_ThirdPersonCharacterCustom OtherActor))
  (Default|LoadGameState _asbp_third_person_character_custom))

(event EventBeginPlay
  (bind _floattrack (Timeline|Timeline PlayFromStart)
    (:Update
      (Transformation|SetRelativeLocation (Variables|Default|Getwall) (Math|Vector|Lerp(Vector) (Variables|/Script/Engine.SceneComponent|GetRelativeLocation (Variables|Default|Getbegin)) (Variables|/Script/Engine.SceneComponent|GetRelativeLocation (Variables|Default|GetEnd)) _floattrack) false false))
    (:Finished
      (Utilities|FlowControl|Delay 0.5)
      (Utilities|FlowControl|FlipFlop ; If A, Reverse from End\nif B, Start from Beginning
        (:A
          (Timeline|Timeline ReverseFromEnd))
        (:B
          (Timeline|Timeline PlayFromStart))))))

(fn ConstructionScript)